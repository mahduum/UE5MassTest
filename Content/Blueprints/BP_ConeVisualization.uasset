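; BP_ConeVisualization is a cone actor that serves as a click-detection and debug visualization test.
; On BeginPlay it enables click events on the first player controller and binds an actor click handler plus an empty capsule hit handler.
; Actor, capsule and static mesh clicks each print their own message, and Tick draws a small debug box at the actor's location.
; A MassAgent component is present but unused in the graph.
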(event `self.ReceiveBeginPlay`
  (add `PrimitiveComponent.OnComponentHit` (`self.Capsule`) (delegate `Component Hit`))
  (add `self.OnClicked` (delegate `OnClicked_Event`))
  (set `PlayerController.bEnableClickEvents` true (`GameplayStatics.GetPlayerController` 0)))

(event `Component Hit`
  (params (HitComponent :type "PrimitiveComponent Object Reference") (OtherActor :type "Actor Object Reference") (OtherComp :type "PrimitiveComponent Object Reference") (NormalImpulse :type "Vector Structure") (Hit :type "HitResult Structure (by ref)")))

(event `OnClicked_Event` :!signature `self.OnClicked`
  (params (TouchedActor :type "Actor Object Reference") (ButtonPressed :type "Key Structure" :default "None"))
  (`KismetSystemLibrary.PrintString` "Cone actor clicked/"))

(event `self.Capsule.OnClicked`
  (params (TouchedComponent :type "PrimitiveComponent Object Reference") (ButtonPressed :type "Key Structure"))
  (`KismetSystemLibrary.PrintString` "Cone capsule clicked!!!"))

(event `self.StaticMesh.OnClicked`
  (params (TouchedComponent :type "PrimitiveComponent Object Reference") (ButtonPressed :type "Key Structure"))
  (`KismetSystemLibrary.PrintString` "Static mesh clicked."))

(event `self.ReceiveTick`
  (params (DeltaSeconds :type "Float (single-precision)"))
  (`KismetSystemLibrary.DrawDebugBox` (`self.K2_GetActorLocation`) (10.0 10.0 10.0) (struct) (struct) 0.1 5.0))

(fn `UserConstructionScript`)