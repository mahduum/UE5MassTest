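; BP_PawnVisualization is a test pawn for visualizing floating pawn movement and actor click input.
; On BeginPlay it binds an OnClicked handler, enables click events, and gives FloatingPawnMovement an initial X velocity with the skeletal mesh as updated component.
; Tick draws a debug box at the actor's location and prints the velocity, while clicks print a message.
; The AddInputVector and static mesh click message nodes are disconnected.
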(event `self.ReceiveBeginPlay`
  (bind _floatingpawnmovement (`self.FloatingPawnMovement`))
  (add `self.OnClicked` (delegate `OnClicked_Event`))
  (set `PlayerController.bEnableClickEvents` true (`GameplayStatics.GetPlayerController` 0))
  (`ActorComponent.SetComponentTickEnabled` _floatingpawnmovement true)
  (set `MovementComponent.Velocity` (500.0 0.0 0.0) _floatingpawnmovement)
  (`MovementComponent.SetUpdatedComponent` _floatingpawnmovement (`self.SkeletalMesh`))
  (`KismetSystemLibrary.PrintString` (`KismetStringLibrary.Conv_VectorToString` (`MovementComponent.Velocity` _floatingpawnmovement)) :!label _label))

(event `OnClicked_Event` :!signature `self.OnClicked`
  (params (TouchedActor :type "Actor Object Reference") (ButtonPressed :type "Key Structure" :default "None"))
  (`KismetSystemLibrary.PrintString` "Cone actor clicked/"))

(event `self.ReceiveTick`
  (params (DeltaSeconds :type "Float (single-precision)"))
  (`KismetSystemLibrary.DrawDebugBox` (`self.K2_GetActorLocation`) (10.0 10.0 10.0) (struct) (struct) 0.1 5.0)
  (goto _label))

(fn `UserConstructionScript`)