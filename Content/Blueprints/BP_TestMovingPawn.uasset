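; Test pawn with a floating movement component, whose only live logic sets the default scene root as the updated component on BeginPlay.
; Tick is empty, so the Blueprint issues no movement itself.
; Disconnected experiments steer toward the current spawn location from PlaceableMassSpawnLocationSubsystem via velocity or input vectors, stopping when close in the velocity version.
; Other unwired fragments print controller and velocity debug info.
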(event `self.ReceiveBeginPlay`
  (`MovementComponent.SetUpdatedComponent` (`self.FloatingPawnMovement`) (`self.DefaultSceneRoot`)))

(event `self.ReceiveTick`
  (params (DeltaSeconds :type "Float (single-precision)")))

(fn `UserConstructionScript`)